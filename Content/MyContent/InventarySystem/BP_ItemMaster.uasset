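; BP_ItemMaster is an item actor that the player picks up with the E key.
; Its sphere collider enables the actor's input for player controller 0 when a BP_MyCharacter begins overlapping and disables it when the overlap ends.
; Pressing E casts the overlapping actor to BP_MyCharacter, passes ItemInfo to its PickUpItem function and destroys the item.
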(event `Key|E`
  (params (Key :type "Key Structure"))
  ;[1 1 1] Pickup
  (:`Pressed`
    (bind _asbp_my_character (cast `/Game/MyContent/BP_MyCharacter` (stale `self.Sphere.OnComponentBeginOverlap` OtherActor)))
    (`/Game/MyContent/BP_MyCharacter.PickUpItem` _asbp_my_character (`self.ItemInfo`))
    (`self.K2_DestroyActor`)))

(event `self.Sphere.OnComponentBeginOverlap`
  (params (OverlappedComponent :type "PrimitiveComponent Object Reference") (OtherActor :type "Actor Object Reference") (OtherComp :type "PrimitiveComponent Object Reference") (OtherBodyIndex :type Integer) (bFromSweep :type Boolean) (SweepResult :type "HitResult Structure (by ref)"))
  ;[1 1 1] Enable and disable input with collider
  (cast `/Game/MyContent/BP_MyCharacter` OtherActor)
  (`self.EnableInput` (`GameplayStatics.GetPlayerController` 0)))

(event `self.Sphere.OnComponentEndOverlap`
  (params (OverlappedComponent :type "PrimitiveComponent Object Reference") (OtherActor :type "Actor Object Reference") (OtherComp :type "PrimitiveComponent Object Reference") (OtherBodyIndex :type Integer))
  ;[1 1 1] Enable and disable input with collider
  (cast `/Game/MyContent/BP_MyCharacter` OtherActor)
  (`self.DisableInput` (`GameplayStatics.GetPlayerController` 0)))

(fn `UserConstructionScript`)